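; BP_Enemy is an enemy Blueprint with top and bottom static meshes whose colors define orange, purple and green variants.
; Three functions, OrangeEnemy, PurpleEnemy and GreenEnemy, each set the two meshes to the pair of primary-color materials that mix into that secondary color.
; Its event graph and construction script are empty, and nothing in the Blueprint calls these functions.
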(event EventBeginPlay)

(event Collision|EventActorBeginOverlap
  (params (OtherActor :type Actor%20Object%20Reference)))

(event EventTick
  (params (DeltaSeconds :type Float%20%28single-precision%29)))

(fn ConstructionScript)

(fn OrangeEnemy
  (Rendering|Material|SetMaterial (Variables|Default|GetTopStaticMesh) 0 "/Game/Environment/M_Red.M_Red")
  (Rendering|Material|SetMaterial (Variables|Default|GetBottomStaticMesh) 0 "/Game/Environment/M_Yellow.M_Yellow"))

(fn PurpleEnemy
  (Rendering|Material|SetMaterial (Variables|Default|GetTopStaticMesh) 0 "/Game/Environment/M_Blue.M_Blue")
  (Rendering|Material|SetMaterial (Variables|Default|GetBottomStaticMesh) 0 "/Game/Environment/M_Red.M_Red"))

(fn GreenEnemy
  (Rendering|Material|SetMaterial (Variables|Default|GetTopStaticMesh) 0 "/Game/Environment/M_Yellow.M_Yellow")
  (Rendering|Material|SetMaterial (Variables|Default|GetBottomStaticMesh) 0 "/Game/Environment/M_Blue.M_Blue"))